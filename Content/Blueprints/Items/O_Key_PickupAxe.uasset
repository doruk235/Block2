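; Axe key-item pickup that adds a journal hint about using the axe to cut a tree stump.
; On any actor overlap it shows a journal popup widget, then appends the hint to the first player pawn's journal entries without checking which actor overlapped.
; It then calls the parent overlap logic, which runs only if the cast to O_PlayerBase succeeds.
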(event EventBeginPlay
  (|CallParentFunction) ; This node is disabled and will not be called.\nDrag off pins to build functionality.
)

(event Collision|EventActorBeginOverlap
  (params (OtherActor :type Actor%20Object%20Reference))
  (bind _returnvalue (UserInterface|CreateWidget "/Game/Blueprints/UI/Journal/UI_JournalPopup.UI_JournalPopup_C"))
  (UserInterface|Viewport|AddtoViewport _returnvalue 0)
  (bind _aso_player_base (Utilities|Casting|CastToO_PlayerBase (Game|Player|GetPlayerPawn 0)))
  (Utilities|Array|Add (Variables|/Game/Blueprints/Player/O_PlayerBase.O_PlayerBase_C|GetJournalEntries _aso_player_base) "I can use the axe to cut that tree stump")
  (|CallParentFunction OtherActor))

(event EventTick
  (params (DeltaSeconds :type Float%20%28single-precision%29))
  (|CallParentFunction DeltaSeconds) ; This node is disabled and will not be called.\nDrag off pins to build functionality.
)

(fn ConstructionScript
  (|CallParentFunction))