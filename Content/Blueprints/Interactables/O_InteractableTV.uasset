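; Interactable TV that plays the intro story audio and holds the player in place while it runs.
; Interacted calls its parent, plays the 2D sound, disables player movement and sets a StartTimer flag.
; Tick polls that flag and, through a DoOnce, waits a fixed 70-second delay before restoring walking.
; The restore and parent Tick call run only once, while Interacted has no repeat guard.
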(event EventBeginPlay
  (|CallParentFunction) ; This node is disabled and will not be called.\nDrag off pins to build functionality.
)

(event Collision|EventActorBeginOverlap
  (params (OtherActor :type Actor%20Object%20Reference))
  (|CallParentFunction OtherActor) ; This node is disabled and will not be called.\nDrag off pins to build functionality.
)

(event EventTick
  (params (DeltaSeconds :type Float%20%28single-precision%29))
  (if (Variables|Default|GetStartTimer)
    (Utilities|FlowControl|DoOnce false
      (:Completed
        (Utilities|FlowControl|Delay 7e+01)
        (bind _aso_player_base (Utilities|Casting|CastToO_PlayerBase (Game|Player|GetPlayerPawn 0))
          (:then
            (Pawn|Components|CharacterMovement|SetMovementMode (Variables|/Script/Engine.Character|GetCharacterMovement _aso_player_base) "MOVE_Walking" 0))
          (:CastFailed
            _))
        (|CallParentFunction DeltaSeconds)))))

(fn ConstructionScript
  (|CallParentFunction))

(fn Interacted
  (|CallParentFunction)
  (Audio|PlaySound2D "/Game/Audio/Intro_Story.Intro_Story" 1.0 1.0 0.0 0 0)
  (bind _aso_player_base (Utilities|Casting|CastToO_PlayerBase (Game|Player|GetPlayerPawn 0)))
  (Pawn|Components|CharacterMovement|DisableMovement (Variables|/Script/Engine.Character|GetCharacterMovement _aso_player_base))
  (Variables|Default|SetStartTimer true))