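; Interactable tree stump that gives the player a clue note, with journal text indicating an axe is needed to cut it down.
; Interacted extends the parent logic and, unless already interacted, spawns an O_Key configured as the note and adds it to the player's inventory.
; ReqsNotMet adds the axe hint to the player's journal and shows a journal popup, guarded by a flag so it happens once.
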(event EventBeginPlay
  (|CallParentFunction) ; This node is disabled and will not be called.\nDrag off pins to build functionality.
)

(event Collision|EventActorBeginOverlap
  (params (OtherActor :type Actor%20Object%20Reference))
  (|CallParentFunction OtherActor) ; This node is disabled and will not be called.\nDrag off pins to build functionality.
)

(event EventTick
  (params (DeltaSeconds :type Float%20%28single-precision%29))
  (|CallParentFunction DeltaSeconds) ; This node is disabled and will not be called.\nDrag off pins to build functionality.
)

(fn ConstructionScript
  (|CallParentFunction))

(fn Interacted
  (|CallParentFunction)
  (if (not (Variables|Default|GetAlreadyInteractedRT))
    (bind _returnvalue (Game|SpawnActorfromClass "/Game/Blueprints/Items/O_Key.O_Key_C" (Math|Transform|MakeTransform "0, 0, 0" "0, 0, 0" "1.000000,1.000000,1.000000") "Undefined" "MultiplyWithRoot" 0 0))
    (Variables|/Game/Blueprints/Items/O_Key.O_Key_C|SetName _returnvalue "Note")
    (Variables|/Game/Blueprints/Items/O_Key.O_Key_C|SetDescription _returnvalue "Go to the house covered in red, then interact with an object of with white and black")
    (Variables|/Game/Blueprints/Items/O_Key.O_Key_C|SetImage _returnvalue "/Game/Blueprints/UI/Inventory/Images/note.note")
    (bind _aso_player_base (Utilities|Casting|CastToO_PlayerBase (Game|Player|GetPlayerPawn 0)))
    (Default|InventoryAdd _aso_player_base _returnvalue)))

(fn ReqsNotMet
  (|CallParentFunction)
  (if (not (Variables|Default|GetAlreadyInteractedRF))
    (bind _aso_player_base (Utilities|Casting|CastToO_PlayerBase (Game|Player|GetPlayerPawn 0)))
    (Utilities|Array|Add (Variables|/Game/Blueprints/Player/O_PlayerBase.O_PlayerBase_C|GetJournalEntries _aso_player_base) "I need to find an axe to cut down this stump")
    (bind _returnvalue (UserInterface|CreateWidget "/Game/Blueprints/UI/Journal/UI_JournalPopup.UI_JournalPopup_C"))
    (UserInterface|Viewport|AddtoViewport _returnvalue 0)
    (Variables|Default|SetAlreadyInteractedRF true)))