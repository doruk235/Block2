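; Interactable door actor that shows a keypad widget and swings open by rotating its DoorEdge component.
; The overridden Interacted creates UI_Keypad for player 0, adds it to the viewport and stores the reference.
; An interaction while that reference is valid rotates the door instantly, removes the widget and sets Opened, which blocks further toggling.
; No code check happens in this Blueprint.
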(event EventBeginPlay
  (|CallParentFunction) ; This node is disabled and will not be called.\nDrag off pins to build functionality.
)

(event Collision|EventActorBeginOverlap
  (params (OtherActor :type Actor%20Object%20Reference))
  (|CallParentFunction OtherActor) ; This node is disabled and will not be called.\nDrag off pins to build functionality.
)

(event EventTick
  (params (DeltaSeconds :type Float%20%28single-precision%29))
  (|CallParentFunction DeltaSeconds) ; This node is disabled and will not be called.\nDrag off pins to build functionality.
)

(fn ConstructionScript
  (|CallParentFunction))

(fn Interacted
  (|CallParentFunction)
  (if (not (Variables|Default|GetOpened))
    (if (Utilities|IsValid (LocalVariables|GetKeypadViewportRef))
      (Transformation|AddLocalRotation (Variables|Default|GetDoorEdge) "0.000000,90.000000,0.000000" false false)
      (Variables|Default|SetOpened true)
      (Widget|RemovefromParent (LocalVariables|GetKeypadViewportRef))
      (else
        (bind _returnvalue (UserInterface|CreateWidget "/Game/Blueprints/UI/Keypad/UI_Keypad.UI_Keypad_C" (Game|GetPlayerController 0)))
        (LocalVariables|SetKeypadViewportRef _returnvalue)
        (UserInterface|Viewport|AddtoViewport _returnvalue 0)))))